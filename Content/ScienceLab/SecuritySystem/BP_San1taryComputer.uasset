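; BP_San1taryComputer is an interactable security-system object in the Science Lab, apparently adapted from door-opening logic.
; Each Interaction alternately plays and reverses a DoorOpen timeline that sets its mesh's relative location.
; Both lerp endpoints are zero, so the mesh gets no travel from the timeline.
; It caches the player's BP_Body on BeginPlay, but the box overlap check against it triggers nothing.
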(event `self.ReceiveBeginPlay`
  ;[0 0.3281 0] InterfaceOpenDoor
  (bind _asbp_body (cast `/Game/EurileneGene/Core/BP_Body` (`GameplayStatics.GetPlayerCharacter` 0)))
  (set `self.As BP Body` _asbp_body))

(event `self.Box.OnComponentBeginOverlap`
  (params (OverlappedComponent :type "PrimitiveComponent Object Reference") (OtherActor :type "Actor Object Reference") (OtherComp :type "PrimitiveComponent Object Reference") (OtherBodyIndex :type Integer) (bFromSweep :type Boolean) (SweepResult :type "HitResult Structure (by ref)"))
  ;[0 0.3281 0] InterfaceOpenDoor
  (if (== OtherActor (`self.As BP Body`))
    _))

(event `/Game/EurileneGene/Core/BPI_Interaction.Interaction`
  ;[0 0.3281 0] InterfaceOpenDoor
  (`/Engine/EditorBlueprintResources/StandardMacros.FlipFlop`
    (:`A`
      (bind (_direction _dooropen) (`Timeline|Timeline` :!label _label)
        (:`Update`
          (`SceneComponent.K2_SetRelativeLocation` (`self.StaticMeshComponent0`) (`KismetMathLibrary.Conv_DoubleToVector` (`KismetMathLibrary.Lerp` 0.0 0.0 _dooropen)) false false))))
    (:`B`
      (goto _label :!via `Reverse`))))

(fn `UserConstructionScript`)